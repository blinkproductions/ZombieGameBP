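; Base weapon Blueprint for an FPS, handling ammo and hitscan shots for the player's FPS character, cached on BeginPlay.
; WeaponFire spends a round and calls CalculateShot, which line-traces from the camera with random per-axis spread and debug drawing.
; The trace result and muzzle socket are not yet used, so no damage or effects occur.
; WeaponReload sets a full magazine and deducts its full size from reserves, alongside two ammo-check helpers.
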(event `self.ReceiveBeginPlay`
  (bind _asfps_character_bp (cast `/Game/Blueprints/FPS_Character_BP` (`GameplayStatics.GetPlayerPawn` 0)))
  (set `self.PlayerRef` _asfps_character_bp))

(fn `CalculateShot`
  (params (Camera :type "CameraComponent Object Reference") (WeaponMesh :type "SceneComponent Object Reference") (WeaponFireSocketName :type Name))
  (locals (LocalCamera :type "CameraComponent Object Reference") (LocalMesh :type "SceneComponent Object Reference") (LocalSocketName :type Name))
  (bind _bulletspread (`self.BulletSpread`))
  (bind (_returnvalue_location _returnvalue_rotation) (`KismetMathLibrary.BreakTransform` (`SceneComponent.K2_GetComponentToWorld` (`local.LocalCamera`))))
  (bind _returnvalue (* _bulletspread -1.0))
  (`|ExecutionSequence`
    (:`then_0`
      (set `local.LocalCamera` Camera)
      (set `local.LocalMesh` WeaponMesh)
      (set `local.LocalSocketName` WeaponFireSocketName))
    (:`then_1`
      (`KismetSystemLibrary.LineTraceSingleForObjects` _returnvalue_location (`KismetMathLibrary.MakeVector` (+ (.x (+ _returnvalue_location (* (`KismetMathLibrary.GetForwardVector` _returnvalue_rotation) 10000.0))) (`KismetMathLibrary.RandomFloatInRange` _returnvalue _bulletspread)) (+ (.y (+ _returnvalue_location (* (`KismetMathLibrary.GetForwardVector` _returnvalue_rotation) 10000.0))) (`KismetMathLibrary.RandomFloatInRange` _returnvalue _bulletspread)) (+ (.z (+ _returnvalue_location (* (`KismetMathLibrary.GetForwardVector` _returnvalue_rotation) 10000.0))) (`KismetMathLibrary.RandomFloatInRange` _returnvalue _bulletspread))) (`|MakeArray` "ObjectTypeQuery1" "ObjectTypeQuery2" :!type "EObjectTypeQuery Enum") false (`|MakeArray` (`GameplayStatics.GetPlayerPawn` 0) :!type "Actor Object Reference") "ForDuration"))))

(fn `HasAmmoInMag`
  (returns (bHasAmmo :type Boolean) (bIsMagFull :type Boolean))
  (bind _currentammo (`self.CurrentAmmo`))
  (return (> _currentammo 0) (== _currentammo (`self.MaxMagAmmo`))))

(fn `HasExtraAmmo`
  (returns (bHasExtraAmmo :type Boolean))
  (return (> (`self.CurrentTotalAmmo`) 0)))

(fn `UserConstructionScript`)

(fn `WeaponFire`
  (set `self.CurrentAmmo` (- (`self.CurrentAmmo`) 1))
  (`self.CalculateShot` (`/Game/Blueprints/FPS_Character_BP.Camera` (`self.PlayerRef`)) (`self.GunMesh`) "MuzzleFlash"))

(fn `WeaponReload`
  (bind _returnvalue (`KismetMathLibrary.Min` (`self.MaxMagAmmo`) (`self.MaxMagAmmo`)))
  (set `self.CurrentAmmo` _returnvalue)
  (set `self.CurrentTotalAmmo` (- (`self.CurrentTotalAmmo`) _returnvalue)))