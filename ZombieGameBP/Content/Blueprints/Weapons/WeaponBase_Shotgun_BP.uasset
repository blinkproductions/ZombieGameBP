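; Shotgun weapon Blueprint that extends parent weapon behavior with shotgun-specific ammo, firing effects and reload timing.
; On BeginPlay it pulls shotgun ammo data from the FPS game instance, then derives reload time from the maximum magazine size.
; Firing calls the parent logic, plays the gun mesh's fire animation and spawns a shell particle effect at the ammo eject socket.
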(event `self.ReceiveBeginPlay`
  (`parent.ReceiveBeginPlay`)
  (bind _asfps_game_instance_bp (cast `/Game/Blueprints/FPS_GameInstance_BP` (`GameplayStatics.GetGameInstance`)))
  (set `self.AmmoData` (`/Game/Blueprints/FPS_GameInstance_BP.ShotgunAmmoData` _asfps_game_instance_bp))
  (`self.SetReloadTime`))

(event `self.WeaponFire`
  (bind (_returnvalue_location _returnvalue_rotation) (`KismetMathLibrary.BreakTransform` (`SceneComponent.GetSocketTransform` (`self.GunMesh`) "AmmoEject" "RTS_World")))
  (`parent.WeaponFire`)
  (`SkeletalMeshComponent.PlayAnimation` (`self.GunMesh`) "/Game/MilitaryWeapSilver/Weapons/Animations/Fire_Shotgun_W.Fire_Shotgun_W" false)
  (`GameplayStatics.SpawnEmitterAtLocation` "/Game/Particles/FX_ShotgunShell.FX_ShotgunShell" _returnvalue_location _returnvalue_rotation))

(event `SetReloadTime`
  (set `self.ReloadTime` (* (`self.MaxMagAmmo`) 0.5)))

(fn `UserConstructionScript`
  (`parent.UserConstructionScript`))