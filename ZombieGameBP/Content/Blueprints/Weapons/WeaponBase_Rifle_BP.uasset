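; Rifle weapon Blueprint that adds automatic fire to a parent weapon class.
; On BeginPlay it takes rifle ammo data from the FPS game instance.
; WeaponFire fires at once, then loops RifleFire on a timer at the automatic fire rate until StopFire clears it.
; Each shot runs the parent fire logic, plays gun and character fire animations, and on empty ammo stops firing and triggers the player's reload.
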(event `self.ReceiveBeginPlay`
  (`parent.ReceiveBeginPlay`)
  (bind _asfps_game_instance_bp (cast `/Game/Blueprints/FPS_GameInstance_BP` (`GameplayStatics.GetGameInstance`)))
  (set `self.AmmoData` (`/Game/Blueprints/FPS_GameInstance_BP.RifleAmmoData` _asfps_game_instance_bp)))

(event `self.WeaponFire`
  (set `self.bIsRifleFiring` true)
  (`self.RifleFire`)
  (bind _returnvalue (`KismetSystemLibrary.K2_SetTimerDelegate` (delegate `RifleFire`) (`self.AutomaticFireRate`) true))
  (set `self.RifleFireTimerHandle` _returnvalue))

(event `RifleFire`
  (if (`self.bIsRifleFiring`)
    (`parent.WeaponFire`)
    (`SkeletalMeshComponent.PlayAnimation` (`self.GunMesh`) "/Game/MilitaryWeapSilver/Weapons/Animations/Fire_Rifle_W.Fire_Rifle_W" false)
    (`/Game/Blueprints/FPS_Character_BP.CharacterFireWeapon` (`self.PlayerRef`) "NewEnumerator1")
    (if (<= (`self.CurrentAmmo`) 0)
      (`self.StopFire`)
      (`/Game/Blueprints/FPS_Character_BP.Reload` (`self.PlayerRef`)))))

(event `self.StopFire`
  (`parent.StopFire`)
  (set `self.bIsRifleFiring` false)
  (`KismetSystemLibrary.K2_ClearAndInvalidateTimerHandle` (`self.RifleFireTimerHandle`)))

(fn `UserConstructionScript`
  (`parent.UserConstructionScript`))